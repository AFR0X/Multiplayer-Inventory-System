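; FogTown player controller that creates the main HUD and inventory widgets, opens and closes the inventory, and spawns dropped items with their quantity.
; Wrapper events forward to CL_ events that build category buttons from DT_Category and manage the UI.
; Slot creation recurses once per category via TemporaryCounter, storing widgets in the Weapons, Food and Potions arrays.
; It then fills a four-column grid with the selected category's slots.
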(event Custom|CL_InitializeWidgets
  ;[1 1 1] Begin play
  (bind _returnvalue (UserInterface|CreateWidget "/Game/UI/WB_Main.WB_Main_C"))
  (bind _output_get (Variables|Default|SetWB_Main _returnvalue))
  (UserInterface|Viewport|AddtoViewport _output_get 0)
  (bind _returnvalue_2 (UserInterface|CreateWidget "/Game/UI/WB_Inventory.WB_Inventory_C"))
  (Variables|Default|SetWB_Inventory _returnvalue_2))

(event Custom|CL_Open/CloseWidget
  (params (Widget :type E_GameWidgets%20Enum :default "NewEnumerator0") (Open :type Boolean))
  ;[1 1 1] Inventory Open And close
  (if Open
    (CallFunction|OpenWidget Widget)
    (else
      (CallFunction|CloseWidget Widget))))

(event Custom|DropItem
  (params (Class :type Actor%20Class%20Reference) (SpawnTransform :type Transform) (Quantity :type Integer))
  (bind _returnvalue (Game|SpawnActorfromClass Class SpawnTransform "AdjustIfPossibleButAlwaysSpawn" "MultiplyWithRoot" 0 0))
  (bind _item (Class|INTItemBase|GetItemRef(Message) _returnvalue))
  (Default|SetItemQuantity _item Quantity))

(event Custom|Open/CloseWidget
  (params (Widget :type E_GameWidgets%20Enum :default "NewEnumerator0") (Open :type Boolean))
  ;[1 1 1] Inventory Open And close
  (CallFunction|CLOpen/CloseWidget Widget Open))

(event Custom|CreateInventoryCategoryWidgets
  ;[1 1 1] Create Invntory Categorys
  (CallFunction|CLCreateInventoryCategoryWidgets))

(event Custom|CL_CreateInventoryCategoryWidgets
  ;[1 1 1] Create Invntory Categorys
  (Widget|Panel|ClearChildren (Variables|/Game/UI/WB_Inventory.WB_Inventory_C|GetVB_Categories (Variables|Default|GetWB_Inventory)))
  (bind _outrownames (DataTable|GetDataTableRowNames "/Game/Blueprints/DataTables/DT_Category.DT_Category"))
  (for _array_element _outrownames
    (bind _returnvalue (UserInterface|CreateWidget "/Game/UI/WB_InventoryCategory.WB_InventoryCategory_C" 0 (.Category (Utilities|Struct|BreakST_InventoryCategory (CallFunction|GetInventoryCategoryInfo (Utilities|String|ToString(Name) _array_element)))) (.CategoryIcon (Utilities|Struct|BreakST_InventoryCategory (CallFunction|GetInventoryCategoryInfo (Utilities|String|ToString(Name) _array_element))))))
    (Class|VerticalBox|AddChildtoVerticalBox (Variables|/Game/UI/WB_Inventory.WB_Inventory_C|GetVB_Categories (Variables|Default|GetWB_Inventory)) _returnvalue)))

(event Custom|CreateInventorySlotWidgets
  (params (Inventory :type AC%20Inventory%20Object%20Reference))
  (CallFunction|CLCreateInventorySlotWidgets Inventory))

(event Custom|CL_CreateInventorySlotWidgets
  (params (Inventory :type AC%20Inventory%20Object%20Reference))
  (bind _weaponscategory (Variables|/Game/Blueprints/Components/AC_Inventory.AC_Inventory_C|GetWeaponsCategory Inventory))
  (bind _foodcategory (Variables|/Game/Blueprints/Components/AC_Inventory.AC_Inventory_C|GetFoodCategory Inventory))
  (bind _potionscategory (Variables|/Game/Blueprints/Components/AC_Inventory.AC_Inventory_C|GetPotionsCategory Inventory))
  (bind _temporarycounter (Variables|Default|GetTemporaryCounter))
  (bind _returnvalue (Utilities|Select :Index _temporarycounter :Option%200 _weaponscategory :Option%201 _foodcategory :Option%202 _potionscategory))
  (bind _outrownames (DataTable|GetDataTableRowNames "/Game/Blueprints/DataTables/DT_Category.DT_Category"))
  (bind _output_get (Variables|Default|SetAmount%20Of%20Categories (- (Utilities|Array|Length _outrownames) 1)))
  (if (<= (Variables|Default|GetTemporaryCounter) _output_get)
    (for _index (range 0 (- (Variables|/Game/Blueprints/Components/AC_Inventory.AC_Inventory_C|GetAmountOfSlots Inventory) 1))
      (bind _returnvalue_2 (UserInterface|CreateWidget "/Game/UI/WB_InventorySlot.WB_InventorySlot_C" 0 _index))
      (Utilities|Array|SetArrayElem _returnvalue _index (Utilities|Struct|MakeST_InventorySlot (.Item (Utilities|Struct|BreakST_InventorySlot (Utilities|Array|Get(acopy) _returnvalue _index))) (.ItemQuantitiy (Utilities|Struct|BreakST_InventorySlot (Utilities|Array|Get(acopy) _returnvalue _index))) _returnvalue_2 _index)))
    (Math|Integer|IncrementInt (Variables|Default|GetTemporaryCounter)
      (:%20%20
        (CallFunction|CreateInventorySlotWidgets Inventory)))
    (else
      (CallFunction|DisyplayInventorySlotWidgets Inventory))))

(event Custom|CL_DisyplayInventorySlotWidgets
  (params (Inventory :type AC%20Inventory%20Object%20Reference))
  (Widget|Panel|ClearChildren (Variables|/Game/UI/WB_Inventory.WB_Inventory_C|GetGRID_Inventory (Variables|Default|GetWB_Inventory)))
  (for _index (range 0 (- (Variables|/Game/Blueprints/Components/AC_Inventory.AC_Inventory_C|GetAmountOfSlots Inventory) 1))
    (Class|GridPanel|AddChildtoGrid (Variables|/Game/UI/WB_Inventory.WB_Inventory_C|GetGRID_Inventory (Variables|Default|GetWB_Inventory)) (.InventorySlot (Utilities|Struct|BreakST_InventorySlot (Utilities|Array|Get(acopy) (Utilities|Select :Index (Variables|/Game/Blueprints/Components/AC_Inventory.AC_Inventory_C|GetSelectedInventoryCategory Inventory) :NewEnumerator0 (Variables|/Game/Blueprints/Components/AC_Inventory.AC_Inventory_C|GetWeaponsCategory Inventory) :NewEnumerator1 (Variables|/Game/Blueprints/Components/AC_Inventory.AC_Inventory_C|GetFoodCategory Inventory) :NewEnumerator2 (Variables|/Game/Blueprints/Components/AC_Inventory.AC_Inventory_C|GetPotionsCategory Inventory)) _index))) (/ _index 4) (Math|Integer|%(Integer) _index 4))
    (Default|UpdateInventorySlotUI (.InventorySlot (Utilities|Struct|BreakST_InventorySlot (Utilities|Array|Get(acopy) (Utilities|Select :Index (Variables|/Game/Blueprints/Components/AC_Inventory.AC_Inventory_C|GetSelectedInventoryCategory Inventory) :NewEnumerator0 (Variables|/Game/Blueprints/Components/AC_Inventory.AC_Inventory_C|GetWeaponsCategory Inventory) :NewEnumerator1 (Variables|/Game/Blueprints/Components/AC_Inventory.AC_Inventory_C|GetFoodCategory Inventory) :NewEnumerator2 (Variables|/Game/Blueprints/Components/AC_Inventory.AC_Inventory_C|GetPotionsCategory Inventory)) _index))) (.Item (Utilities|Struct|BreakST_InventorySlot (Utilities|Array|Get(acopy) (Utilities|Select :Index (Variables|/Game/Blueprints/Components/AC_Inventory.AC_Inventory_C|GetSelectedInventoryCategory Inventory) :NewEnumerator0 (Variables|/Game/Blueprints/Components/AC_Inventory.AC_Inventory_C|GetWeaponsCategory Inventory) :NewEnumerator1 (Variables|/Game/Blueprints/Components/AC_Inventory.AC_Inventory_C|GetFoodCategory Inventory) :NewEnumerator2 (Variables|/Game/Blueprints/Components/AC_Inventory.AC_Inventory_C|GetPotionsCategory Inventory)) _index))) (.ItemQuantitiy (Utilities|Struct|BreakST_InventorySlot (Utilities|Array|Get(acopy) (Utilities|Select :Index (Variables|/Game/Blueprints/Components/AC_Inventory.AC_Inventory_C|GetSelectedInventoryCategory Inventory) :NewEnumerator0 (Variables|/Game/Blueprints/Components/AC_Inventory.AC_Inventory_C|GetWeaponsCategory Inventory) :NewEnumerator1 (Variables|/Game/Blueprints/Components/AC_Inventory.AC_Inventory_C|GetFoodCategory Inventory) :NewEnumerator2 (Variables|/Game/Blueprints/Components/AC_Inventory.AC_Inventory_C|GetPotionsCategory Inventory)) _index))))))

(event Custom|DisyplayInventorySlotWidgets
  (params (Inventory :type AC%20Inventory%20Object%20Reference))
  (CallFunction|CLDisyplayInventorySlotWidgets Inventory))

(event EventBeginPlay
  ;[1 1 1] Begin play
  (CallFunction|CLInitializeWidgets)
  (CallFunction|Open/CloseWidget "NewEnumerator0" false))

(fn ConstructionScript)

(fn OpenWidget
  (params (Widget :type E_GameWidgets%20Enum :default "NewEnumerator0"))
  (switch Utilities|FlowControl|Switch|SwitchonE_GameWidgets Widget
    (:NewEnumerator0
      (Variables|Default|GetWB_Inventory
        (:then
          _)
        (:else
          (bind _returnvalue (UserInterface|CreateWidget "/Game/UI/WB_Inventory.WB_Inventory_C"))
          (bind _output_get (Variables|Default|SetWB_Inventory _returnvalue))))
      (UserInterface|Viewport|AddtoViewport _output_get 0)
      (Variables|Default|SetbInventoryIsOpen true))))

(fn CloseWidget
  (params (Widget :type E_GameWidgets%20Enum :default "NewEnumerator0"))
  (switch Utilities|FlowControl|Switch|SwitchonE_GameWidgets Widget
    (:NewEnumerator0
      (bind _wb_inventory (Variables|Default|GetWB_Inventory)
        (:then
          (Widget|RemovefromParent _wb_inventory)
          (Variables|Default|SetbInventoryIsOpen false))
        (:else)))))

(fn GetPlayerControllerRef
  (return self))