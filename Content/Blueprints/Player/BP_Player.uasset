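; BP_Player is the player pawn, handling movement, yaw-only look, inventory toggling and item looting through Enhanced Input.
; On BeginPlay it adds the default mapping context, initializes its ACInventory component and has the player controller build inventory widgets.
; The inventory action opens or closes that UI with sound.
; Server-prefixed loot events add the first overlapping BP_ItemBase to ACInventory, using message calls to fetch references.
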(event Custom|OpenInventory
  (bind _player_controller (Variables|Default|GetPlayer%20Controller))
  ;[1 1 1] Open Inv
  (if (Variables|/Game/Blueprints/PC_FogTown.PC_FogTown_C|GetbInventoryIsOpen _player_controller)
    (Default|Open/CloseWidget _player_controller "NewEnumerator0" false)
    (Audio|PlaySound2D "/Game/Audio/SFX_CloseInventory_Cue.SFX_CloseInventory_Cue" 1.0 1.0 0.0 0 0)
    (else
      (Default|Open/CloseWidget _player_controller "NewEnumerator0" true)
      (Audio|PlaySound2D "/Game/Audio/SFX_OpenInventory_Cue.SFX_OpenInventory_Cue" 1.0 1.0 0.0 0 0))))

(event Custom|SRV_Loot
  (bind _overlappingactors (Collision|GetOverlappingActors "/Game/Blueprints/Items/BP_ItemBase.BP_ItemBase_C" :!class /Script/Engine.Actor))
  (if (> (Utilities|Array|Length _overlappingactors) 0)
    (bind _item (Class|INTItemBase|GetItemRef(Message) (Utilities|Array|Get(acopy) _overlappingactors)))
    (Default|AddtoInventory (Variables|Default|GetAC_Inventory) _item)))

(event Custom|SRV_RelootItem
  (Default|AddtoInventory (Variables|Default|GetAC_Inventory) (stale Custom|SRV_Loot _item)))

(event Input|EnhancedActionEvents|EnhancedInputActionIA_Movement
  (params (ActionValue :type Vector%202D%20Structure) (ElapsedSeconds :type Float%20%28double-precision%29) (TriggeredSeconds :type Float%20%28double-precision%29) (InputAction :type Input%20Action%20Object%20Reference :default "/Game/Blueprints/Player/IA_Movement.IA_Movement"))
  (Pawn|Input|AddMovementInput (Transformation|GetActorForwardVector) (.x ActionValue) false)
  (Pawn|Input|AddMovementInput (Transformation|GetActorRightVector) (.y ActionValue) false))

(event Input|EnhancedActionEvents|EnhancedInputActionIA_Inventory
  (params (ActionValue :type Boolean) (ElapsedSeconds :type Float%20%28double-precision%29) (TriggeredSeconds :type Float%20%28double-precision%29) (InputAction :type Input%20Action%20Object%20Reference :default "/Game/Blueprints/Player/IA_Inventory.IA_Inventory"))
  (bind _player_controller (Variables|Default|GetPlayer%20Controller))
  ;[1 1 1] Open Inv
  (if (Variables|/Game/Blueprints/PC_FogTown.PC_FogTown_C|GetbInventoryIsOpen _player_controller)
    (Default|Open/CloseWidget _player_controller "NewEnumerator0" false)
    (Audio|PlaySound2D "/Game/Audio/SFX_CloseInventory_Cue.SFX_CloseInventory_Cue" 1.0 1.0 0.0 0 0)
    (else
      (Default|Open/CloseWidget _player_controller "NewEnumerator0" true)
      (Audio|PlaySound2D "/Game/Audio/SFX_OpenInventory_Cue.SFX_OpenInventory_Cue" 1.0 1.0 0.0 0 0))))

(event Input|EnhancedActionEvents|EnhancedInputActionIA_Look
  (params (ActionValue :type Float%20%28double-precision%29) (ElapsedSeconds :type Float%20%28double-precision%29) (TriggeredSeconds :type Float%20%28double-precision%29) (InputAction :type Input%20Action%20Object%20Reference :default "/Game/Blueprints/Player/IA_Look.IA_Look"))
  (Pawn|Input|AddControllerYawInput ActionValue))

(event Input|EnhancedActionEvents|EnhancedInputActionIA_Loot
  (params (ActionValue :type Boolean) (ElapsedSeconds :type Float%20%28double-precision%29) (TriggeredSeconds :type Float%20%28double-precision%29) (InputAction :type Input%20Action%20Object%20Reference :default "/Game/Blueprints/Player/IA_Loot.IA_Loot"))
  (:Triggered
    (CallFunction|SRVLoot)))

(event EventBeginPlay
  (bind _playercontroller (Class|INTPlayerController|GetPlayerControllerRef(Message) (Pawn|GetController)))
  (bind _output_get (Variables|Default|SetPlayer%20Controller _playercontroller))
  (Utilities|IsValid _output_get
    (:Is%20Valid
      (bind _aspc_fog_town (Utilities|Casting|CastToPC_FogTown (Pawn|GetController)))
      (Input|AddMappingContext (PlayerController|LocalPlayerSubsystems|GetEnhancedInputLocalPlayerSubsystem _aspc_fog_town) "/Game/Blueprints/Player/IMC_Default.IMC_Default" 0 "(bIgnoreAllPressedKeysUntilRelease=True,bForceImmediately=False,bNotifyUserSettings=False)")
      (Default|InitializeInventory (Variables|Default|GetAC_Inventory))
      (Default|CreateInventoryCategoryWidgets (Variables|Default|GetPlayer%20Controller))
      (Default|CreateInventorySlotWidgets (Variables|Default|GetPlayer%20Controller) (Variables|Default|GetAC_Inventory)))))

(fn ConstructionScript)

(fn GetPlayerRef
  (return self))