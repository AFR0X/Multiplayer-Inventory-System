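; Inventory component that stores looted items in fixed-size Weapons, Food and Potions slot arrays and refreshes slot widgets for the selected category.
; Client events handle setup, category switching and adding items, while server events handle quantity changes, looted-item destruction and drop requests through the GameMode.
; Stackable items fill partial stacks through FindPartialStack before CreateNewStack takes empty slots.
; Oversized new stacks trigger a server re-loot of the remainder.
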(event Custom|CL_InitializeInventory
  (bind _amountofslots (Variables|Default|GetAmountOfSlots))
  ;[1 1 1] resize Inventory
  (Utilities|Array|Resize (Variables|Default|GetWeaponsCategory) _amountofslots)
  (Utilities|Array|Resize (Variables|Default|GetFoodCategory) _amountofslots)
  (Utilities|Array|Resize (Variables|Default|GetPotionsCategory) _amountofslots))

(event Custom|InitializeInventory
  ;[1 1 1] resize Inventory
  (CallFunction|CLInitializeInventory))

(event Custom|SRV_DestroyLootedItem
  (params (Item :type BP%20Item%20Base%20Object%20Reference) (Destroy%20Item :type Boolean))
  (Default|DestroyLootedItem Item Destroy%20Item))

(event Custom|DropItem
  (params (PlayerController :type PC%20Fog%20Town%20Object%20Reference) (Class :type Actor%20Class%20Reference) (Quantity :type Integer) (Location :type Vector))
  (CallFunction|SRVDropItem PlayerController Class Quantity Location))

(event Custom|SRV_DropItem
  (params (PlayerController :type PC%20Fog%20Town%20Object%20Reference) (Class :type Actor%20Class%20Reference) (Quantity :type Integer) (Location :type Vector))
  (bind _gamemode (Class|INTGameMode|GetGameModeRef(Message) (Game|GetGameMode)))
  (Default|RequestDropItem _gamemode PlayerController Class Quantity Location))

(event Custom|SetSelectionInventyoryCategory
  (params (SelectedInventoryCategory :type E_ItemCategory%20Enum :default "NewEnumerator0"))
  ;[1 1 1] Change Category
  (CallFunction|CLSetSelectionInventyoryCategory SelectedInventoryCategory))

(event Custom|CL_SetSelectionInventyoryCategory
  (params (SelectedInventoryCategory :type E_ItemCategory%20Enum :default "NewEnumerator0"))
  ;[1 1 1] Change Category
  (Variables|Default|SetSelectedInventoryCategory SelectedInventoryCategory)
  (bind _player (Class|INTPlayer|GetPlayerRef(Message) (Components|GetOwner)))
  (Default|DisyplayInventorySlotWidgets (Variables|/Game/Blueprints/Player/BP_Player.BP_Player_C|GetPlayer%20Controller _player) (Variables|/Game/Blueprints/Player/BP_Player.BP_Player_C|GetAC_Inventory _player)))

(event Custom|AddToInventory
  (params (Item :type BP%20Item%20Base%20Object%20Reference))
  (CallFunction|CLAddtoInventory Item))

(event Custom|CL_AddToInventory
  (params (Item :type BP%20Item%20Base%20Object%20Reference))
  (bind _output_get (Variables|Default|SetItemAddRef Item))
  (bind _output_get_2 (Variables|Default|SetItemToAdd (CallFunction|GetItemInfo (Variables|/Game/Blueprints/Items/BP_ItemBase.BP_ItemBase_C|GetItemName _output_get))))
  (if (Utilities|Struct|BreakST_ItemInfo _output_get_2)
    (bind (_itemtoadd _quantityadd _inventoryslot _slotindex _inventory) (Utilities|FindPartialStack :!label _label)
      (:Found
        (if (<= _quantityadd (Utilities|Struct|BreakST_ItemInfo (Variables|Default|GetItemToAdd)))
          (CallFunction|AddItemtoInventory _itemtoadd _quantityadd _inventoryslot _slotindex _inventory)
          (Variables|Default|SetbHasToCreateStack false)
          (goto _label Break%20Loop)
          (else
            (CallFunction|SetNewItemQuantity (Variables|Default|GetItemAddRef) (- (Variables|/Game/Blueprints/Items/BP_ItemBase.BP_ItemBase_C|GetQuantity (Variables|Default|GetItemAddRef)) (Utilities|Struct|BreakST_ItemInfo (Variables|Default|GetItemToAdd))))
            (CallFunction|AddItemtoInventory _itemtoadd (Utilities|Struct|BreakST_ItemInfo (Variables|Default|GetItemToAdd)) _inventoryslot _slotindex _inventory)
            (Variables|Default|SetbHasToCreateStack true)
            (goto _label Break%20Loop))))
      (:Not%20Found
        (Utilities|FlowControl|Delay 0.05)
        (bind (_itemtoadd_2 _quantitiyadd _inventoryslot_2 _slotindex_2 _inventory_2) (Utilities|CreateNewStack :!label _label_2)
          (:Stack
            (CallFunction|AddItemtoInventory _itemtoadd_2 _quantitiyadd _inventoryslot_2 _slotindex_2 _inventory_2)
            (goto _label_2 BreakLoop))
          (:LoopComplete
            (Audio|PlaySound2D "/Game/Audio/SFX_LootItem_Cue.SFX_LootItem_Cue" 1.0 1.0 0.0 0 0)
            (CallFunction|DestroyLootedItem (Variables|Default|GetItemAddRef) true))))
      (:Loop%20Completed
        (Audio|PlaySound2D "/Game/Audio/SFX_LootItem_Cue.SFX_LootItem_Cue" 1.0 1.0 0.0 0 0)
        (CallFunction|DestroyLootedItem (Variables|Default|GetItemAddRef) true)))
    (else
      (goto _label_2))))

(event Custom|SetNewItemQuantity
  (params (Item :type BP%20Item%20Base%20Object%20Reference) (Quantity :type Integer))
  (CallFunction|SRVSetNewItemQuantity Item Quantity))

(event Custom|SRV_SetNewItemQuantity
  (params (Item :type BP%20Item%20Base%20Object%20Reference) (Quantity :type Integer))
  (Default|SetItemQuantity Item Quantity))

(event Custom|DestroyLootedItem
  (params (Item :type BP%20Item%20Base%20Object%20Reference) (Destroy%20Item :type Boolean))
  (CallFunction|SRVDestroyLootedItem Item Destroy%20Item))

(event EventBeginPlay)

(event EventTick
  (params (DeltaSeconds :type Float%20%28single-precision%29)))

(fn AddItemtoInventory
  (params (Item :type ST%20Item%20Info%20Structure) (Quantity :type Integer) (InventorySlot :type WB%20Inventory%20Slot%20Object%20Reference) (SlotIndex :type Integer) (Inventory :type Array%20of%20ST%20Inventory%20Slot%20Structures))
  (Utilities|Array|SetArrayElem Inventory SlotIndex (Utilities|Struct|MakeST_InventorySlot Item Quantity InventorySlot SlotIndex))
  (if (Utilities|Enum|Equal(Enum) (Utilities|Struct|BreakST_ItemInfo Item) (Variables|Default|GetSelectedInventoryCategory))
    (Default|UpdateInventorySlotUI InventorySlot Item Quantity)))