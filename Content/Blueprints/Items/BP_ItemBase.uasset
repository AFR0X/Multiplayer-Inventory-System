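; Base item actor for lootable world pickups, with a static mesh that starts simulating physics on BeginPlay.
; Events set the item's quantity and its destroyed flag, and GetItemRef returns the actor itself.
; Looting removal runs through replication: the destroyed flag's RepNotify destroys the actor when the flag is true.
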(event Custom|SetItemQuantity
  (params (Quantity :type Integer))
  (Variables|Default|SetQuantity Quantity))

(event Custom|DestroyLootedItem
  (params (bDestroyedItem :type Boolean))
  (Variables|Default|SetbDestroyedItem bDestroyedItem))

(event EventBeginPlay
  (Physics|SetSimulatePhysics (Variables|Default|GetStaticMesh) true))

(fn ConstructionScript)

(fn OnRepBDestroyedItem
  (if (Variables|Default|GetbDestroyedItem)
    (Actor|DestroyActor)))

(fn GetItemRef
  (return self))